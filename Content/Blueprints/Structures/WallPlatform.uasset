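; WallPlatform is a structure that blocks or allows passage based on whether a wall of its assigned class is walkable.
; On BeginPlay it finds the first WallManager in the level and binds to its wall state change event.
; When the changed wall's class exactly matches WallClass, it disables BlockingCollision if that wall is walkable and enables query and physics collision otherwise.
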(event `self.ReceiveBeginPlay`
  (bind _outactors (`GameplayStatics.GetAllActorsOfClass` "/Game/Blueprints/WallManager.WallManager_C"))
  (add `/Game/Blueprints/WallManager.WallStateChanged` (`|GetArrayItem` _outactors) (delegate `On Wall State Changed`)))

(event `On Wall State Changed`
  (params (Wall :type "/Game/Blueprints/Structures/Wall Object Reference"))
  (if (== (`GameplayStatics.GetObjectClass` Wall) (`self.Wall Class`))
    (if (`/Game/Blueprints/Structures/Wall.Walkable` Wall)
      (`PrimitiveComponent.SetCollisionEnabled` (`self.BlockingCollision`) "NoCollision")
      (else
        (`PrimitiveComponent.SetCollisionEnabled` (`self.BlockingCollision`) "QueryAndPhysics")))))

(fn `UserConstructionScript`)