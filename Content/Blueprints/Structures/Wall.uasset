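; Destructible wall of two mesh halves that a BuilderSlime can repair for StickyGoop.
; Damage plays a random sound and timeline shake, breaking the top at a health threshold and the bottom at zero via radius damage.
; Interaction runs a Job with looping work audio; finishing deducts goop and has WallManager respawn the wall.
; Healing can reveal a cost widget, and Y and V keys directly trigger top break and shake.
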(event `Key|Y`
  (params (Key :type "Key Structure"))
  (:`Pressed`
    (`self.Break Top`)))

(event `Break Top`
  (`KismetSystemLibrary.Delay` 0.1)
  (`DestructibleComponent.ApplyRadiusDamage` (`self.TopHalf`) 5000.0 (`self.TopDamageLocation`) 5000.0 5000.0 true)
  (`PrimitiveComponent.SetCollisionEnabled` (`self.OnBreakWall`) "QueryAndPhysics"))

(event `Break Bottom`
  (`DestructibleComponent.ApplyRadiusDamage` (`self.BottomHalf`) 3000.0 (`self.Bottom Damage Location`) 3000.0 3000.0 true))

(event `Restore`
  (bind _outactors (`GameplayStatics.GetAllActorsOfClass` "/Game/Blueprints/WallManager.WallManager_C"))
  (`/Game/Blueprints/WallManager.Respawn` (`|GetArrayItem` _outactors) (`GameplayStatics.GetObjectClass` self) 0.1 self))

(event `self.ReceiveBeginPlay`
  (`parent.ReceiveBeginPlay`)
  (`/Game/Blueprints/Components/TetrisRandomizer.SetArraySize` (`self.DamageRandomizer`) (`KismetArrayLibrary.Array_Length` (`self.DamageSounds`)))
  (`KismetSystemLibrary.Delay` 0.0)
  (`PrimitiveComponent.SetMaterial` (`self.TopHalf`) 0 (`self.Top Material`))
  (`PrimitiveComponent.SetMaterial` (`self.BottomHalf`) 0 (`self.Bottom Material`)))

(event `self.Job.OnBegin`
  (`AudioComponent.FadeIn` (`self.HammerSound`) 0.2 0.3 0.0)
  (`AudioComponent.FadeIn` (`self.MachineSound`) 0.2 0.15 0.0))

(event `self.Health.OnKilled`)

(event `self.Job.OnFinish`
  (bind _asslime_mode (cast `/Game/Blueprints/SlimeMode` (`GameplayStatics.GetGameMode`) :!pure true))
  (set `/Game/Blueprints/SlimeMode.StickyGoop` (- (`/Game/Blueprints/SlimeMode.StickyGoop` _asslime_mode) (`.Cost_2_5E91E0484C4DD3BFB5F332A64E2971B3` (break `/Game/Blueprints/Enums/CostStruct` (`self.Cost`)))) _asslime_mode)
  (`self.Restore`)
  (`/Engine/EditorBlueprintResources/StandardMacros.IsValid` self
    (:`Is Valid`
      (`AudioComponent.FadeOut` (`self.HammerSound`) 0.2 0.0 :!label _label)
      (`AudioComponent.FadeOut` (`self.MachineSound`) 0.2 0.0))))

(event `self.Job.OnCancel`
  (goto _label))

(event `self.Health.OnDamaged`
  (params (Amount :type "Float (single-precision)"))
  (bind _index (`/Game/Blueprints/Components/TetrisRandomizer.PickIndex` (`self.DamageRandomizer`)))
  (`GameplayStatics.PlaySoundAtLocation` (`|GetArrayItem` (`self.DamageSounds`) _index) (`self.K2_GetActorLocation` self) (struct) 0.55 1.0 0.0 null null null)
  (`self.Shake`)
  (if (<= (`/Game/Blueprints/Components/Health.Health` (`self.Health`)) 0.0)
    (`/Engine/EditorBlueprintResources/StandardMacros.DoOnce` false
      (:`Completed`
        (`self.Break Bottom`)))
    (elif (<= (`/Game/Blueprints/Components/Health.Health` (`self.Health`)) 75.0)
      (`/Engine/EditorBlueprintResources/StandardMacros.DoOnce` false
        (:`Completed`
          (`self.Break Top`))))))

(event `self.Health.OnHealed`
  (params (Amount :type "Float (single-precision)"))
  (`self.ShowCostWidget`))

(event `Shake`
  (bind (_direction _newtrack_0) (`Timeline|ShakeTimeline` :!via `PlayFromStart`)
    (:`Update`
      (`|ExecutionSequence`
        (:`then_0`
          (`SceneComponent.K2_SetRelativeLocation` (`self.BottomHalf`) (`KismetMathLibrary.MakeVector` 0.0 _newtrack_0) false false))
        (:`then_1`
          (`SceneComponent.K2_SetRelativeLocation` (`self.TopHalf`) (`KismetMathLibrary.MakeVector` 0.0 _newtrack_0) false false))))))

(event `self.ShowCostWidget`
  (bind _health (`self.Health`))
  (bind (_asslime_mode _bsuccess) (cast `/Game/Blueprints/SlimeMode` (`GameplayStatics.GetGameMode`) :!pure true))
  (if (and _bsuccess (== (`/Game/Blueprints/SlimeMode.PossessedChar` _asslime_mode) (`self.PlayerIndexWanted`)) (< (`/Game/Blueprints/Components/Health.Health` _health) (`/Game/Blueprints/Components/Health.MaxHealth` _health)))
    (`Widget.SetVisibility` (`self.CostWidget`) "Visible")
    (`/Game/Blueprints/UI/CostWidget.UpdateCost` (`self.CostWidget`) (`self.Cost`) "")))

(event `Key|V`
  (params (Key :type "Key Structure"))
  (:`Pressed`
    (`self.Shake`)))

(fn `CanInteract`
  (params (InteractingActor :type "/Game/Blueprints/Units/TestPawn Object Reference"))
  (returns (CanInteract :type Boolean))
  (bind _health (`self.Health`))
  (cast `/Game/Blueprints/Units/BuilderSlime` InteractingActor
    (:`then`
      (if (and (< (`/Game/Blueprints/Components/Health.Health` _health) (`/Game/Blueprints/Components/Health.MaxHealth` _health)) (>= (`/Game/Blueprints/SlimeMode.StickyGoop` (cast `/Game/Blueprints/SlimeMode` (`GameplayStatics.GetGameMode`) :!pure true)) (`self.Goop Cost`)))
        (return true)
        (else
          (return false))))
    (:`CastFailed`
      (return false))))

(fn `InteractPressed`
  (params (`Interacting Actor` :type "/Game/Blueprints/Units/TestPawn Object Reference"))
  (returns (Success :type Boolean) (Job :type "/Game/Blueprints/Components/Job Object Reference"))
  (bind _caninteract (`self.CanInteract` `Interacting Actor`))
  (if _caninteract
    (`/Game/Blueprints/Components/Job.Begin` (`self.Job`))
    (return true (`self.Job`))
    (else
      (return false null))))

(fn `UserConstructionScript`
  (`DestructibleComponent.SetDestructibleMesh` (`self.TopHalf`) (`self.Top Mesh`))
  (`DestructibleComponent.SetDestructibleMesh` (`self.BottomHalf`) (`self.Bottom Mesh`))
  (`PrimitiveComponent.SetMaterial` (`self.TopHalf`) 0 (`self.Top Material`))
  (`PrimitiveComponent.SetMaterial` (`self.BottomHalf`) 0 (`self.Bottom Material`)))