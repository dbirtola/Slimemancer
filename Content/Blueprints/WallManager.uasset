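; WallManager is a manager Blueprint that respawns walls and relays their state changes through its own WallStateChanged dispatcher.
; On BeginPlay it binds to the OnWallStateChanged event of every Wall in the level and rebroadcasts each change with its second parameter, dropping the walkable flag.
; Respawn destroys a wall, waits a given delay, spawns the given class at the saved transform, then binds and broadcasts the new wall.
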(event `Respawn`
  (params (WallClass :type "/Game/Blueprints/Structures/Wall Class Reference") (Delay :type "Float (double-precision)") (OriginalWall :type "/Game/Blueprints/Structures/Wall Object Reference"))
  (set `self.Transform` (`self.GetTransform` OriginalWall))
  (`self.K2_DestroyActor` OriginalWall)
  (`KismetSystemLibrary.Delay` Delay)
  (bind _returnvalue (`|SpawnActorFromClass` WallClass (`self.Transform`) "Undefined" "OverrideRootScale" null null))
  (add `/Game/Blueprints/Structures/Wall.OnWallStateChanged` _returnvalue (delegate `On Wall state Changed`))
  (`self.WallStateChanged` _returnvalue))

(event `self.ReceiveBeginPlay`
  (bind _outactors (`GameplayStatics.GetAllActorsOfClass` "/Game/Blueprints/Structures/Wall.Wall_C"))
  (for _array_element _outactors
    (add `/Game/Blueprints/Structures/Wall.OnWallStateChanged` _array_element (delegate `On Wall state Changed`))))

(event `On Wall state Changed`
  (params (Walkable :type Boolean) (NewParam :type "/Game/Blueprints/Structures/Wall Object Reference"))
  (`self.WallStateChanged` NewParam))

(fn `UserConstructionScript`)