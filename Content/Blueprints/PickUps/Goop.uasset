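; Goop pickup that a TestPawn collects by walking into its Box trigger.
; On overlap it passes its GoopValue to the SlimeMode game mode through CollectGoop with a popup, then destroys itself.
; The interaction functions CanInteract and InteractPressed always return false, so collection happens only through overlap.
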(event `self.Box.OnComponentBeginOverlap`
  (params (OverlappedComponent :type "PrimitiveComponent Object Reference") (OtherActor :type "Actor Object Reference") (OtherComp :type "PrimitiveComponent Object Reference") (OtherBodyIndex :type Integer) (bFromSweep :type Boolean) (SweepResult :type "HitResult Structure (by ref)"))
  (cast `/Game/Blueprints/Units/TestPawn` OtherActor)
  (bind _asslime_mode (cast `/Game/Blueprints/SlimeMode` (`GameplayStatics.GetGameMode`)))
  (`/Game/Blueprints/SlimeMode.CollectGoop` _asslime_mode (`self.Goop Value`) true self)
  (`self.K2_DestroyActor`))

(fn `CanInteract`
  (params (InteractingActor :type "/Game/Blueprints/Units/TestPawn Object Reference"))
  (returns (CanInteract :type Boolean))
  (return false))

(fn `InteractPressed`
  (params (`Interacting Actor` :type "/Game/Blueprints/Units/TestPawn Object Reference"))
  (returns (Success :type Boolean) (Job :type "/Game/Blueprints/Components/Job Object Reference"))
  (return false null))

(fn `UserConstructionScript`)