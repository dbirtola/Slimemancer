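; Slime unit AI that marches on the nearest targetable Wall, heading for the QueenSlime if none is found or once that wall is killed.
; TestPawns other than FighterSlime entering its detection range become chase targets, and it resumes the march when none remain.
; Tick applies cooldown-gated overlap damage to one Health faction, faces velocity and fades walk audio with movement.
; Death plays a sound, spawns Goop and destroys the actor.
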(event `self.ReceiveTick`
  (params (DeltaSeconds :type "Float (single-precision)"))
  (bind _returnvalue (`self.GetVelocity`))
  (bind _walkcycle (`self.WalkCycle`))
  (bind _returnvalue_2 (`KismetMathLibrary.VSize` (`self.GetVelocity`)))
  (`|ExecutionSequence`
    (:`then_0`
      (`/Engine/EditorBlueprintResources/StandardMacros.DoOnce` false :!label _label
        (:`Completed`
          (for _array_element (`PrimitiveComponent.GetOverlappingActors` (`self.Damage Collider`) "/Script/Engine.Actor")
            (bind _returnvalue_3 (`self.GetComponentByClass` _array_element "/Game/BluePrints/Health.Health_C"))
            (`/Engine/EditorBlueprintResources/StandardMacros.IsValid` _returnvalue_3
              (:`Is Valid`
                (if (`|EnumEquality` (`/Game/BluePrints/Health.Faction` _returnvalue_3) "NewEnumerator0")
                  (`/Game/BluePrints/Health.Damage` _returnvalue_3 (`self.Slime Damage`))))))
          (`KismetSystemLibrary.Delay` (`self.Attack Cooldown`))
          (goto _label :!via `Reset`))))
    (:`then_1`
      (if (> (`KismetMathLibrary.VSizeXY` _returnvalue) 5.0)
        (`self.K2_SetActorRotation` (`KismetMathLibrary.MakeRotFromX` _returnvalue))))
    (:`then_2`
      (`/Engine/EditorBlueprintResources/StandardMacros.DoOnce` false
        (:`Completed`
          (`AudioComponent.FadeOut` _walkcycle 0.1 0.0 :!label _label_2)
          (if (<= _returnvalue_2 0.1) :!label _label_3
            (`KismetSystemLibrary.Delay` 0.0)
            (goto _label_3)
            (else
              (`AudioComponent.FadeIn` _walkcycle 0.2 0.5 0.0)
              (if (> _returnvalue_2 0.1) :!label _label_4
                (`KismetSystemLibrary.Delay` 0.0)
                (goto _label_4)
                (else
                  (goto _label_2))))))))))

(event `self.ReceiveBeginPlay`
  (bind _returnvalue (`self.K2_GetActorLocation`))
  (bind _outactors (`GameplayStatics.GetAllActorsOfClass` "/Game/BluePrints/Structures/Wall.Wall_C" :!label _label_5))
  (bind (_arrayindex _arrayelement) (`/Engine/EditorBlueprintResources/StandardMacros.ReverseForEachLoop` _outactors)
    (:`LoopBody`
      (if (not (`/Game/BluePrints/Structures/Wall.Targetable` _arrayelement))
        (`KismetArrayLibrary.Array_RemoveItem` _outactors _arrayelement)))
    (:`Completed`
      (bind _closest_actor (`/Game/BluePrints/Libraries/HelperFunctions.GetClosestActorToActors` self _outactors))
      (bind _aswall (cast `/Game/BluePrints/Structures/Wall` _closest_actor)
        (:`then`
          (if (>= (`/Game/BluePrints/Health.Health` (`/Game/BluePrints/Structures/Wall.Health` _aswall)) 0.0)
            (bind _returnvalue_2 (- (`self.K2_GetActorLocation` _aswall) (`self.K2_GetActorLocation`)))
            (`AIController.MoveToLocation` (`AIBlueprintHelperLibrary.GetAIController` self) (+ (`self.K2_GetActorLocation`) (* (`KismetMathLibrary.Normal` _returnvalue_2) (- (`KismetMathLibrary.VSize` _returnvalue_2) 200.0))) 25.0 true true false true null true)
            (add `/Game/BluePrints/Health.OnKilled` (`self.GetComponentByClass` _aswall "/Game/BluePrints/Health.Health_C") (delegate `On Gate Killed`))))
        (:`CastFailed`
          (bind _outactors_2 (`GameplayStatics.GetAllActorsOfClass` "/Game/BluePrints/Units/QueenSlime.QueenSlime_C" :!label _label_6))
          (bind _output (`|GetArrayItem` _outactors_2))
          (`/Engine/EditorBlueprintResources/StandardMacros.IsValid` _output
            (:`Is Valid`
              (bind _returnvalue_3 (- (`self.K2_GetActorLocation` _output) _returnvalue))
              (bind _returnvalue_4 (`AIController.MoveToLocation` (`AIBlueprintHelperLibrary.GetAIController` self) (+ _returnvalue (* (`KismetMathLibrary.Normal` _returnvalue_3) (- (`KismetMathLibrary.VSize` _returnvalue_3) 40.0))) 25.0 true true true true null true))
              (`KismetSystemLibrary.PrintString` (`|GetEnumeratorNameAsString` _returnvalue_4)))))))))

(event `On Gate Killed`
  (goto _label_6))

(event `self.Health.OnKilled`
  (`KismetSystemLibrary.PrintString` "Im dead now")
  (`GameplayStatics.PlaySoundAtLocation` "/Game/Sounds/slime/disgruntledSlime.disgruntledSlime" (`self.K2_GetActorLocation` self) (struct) 1.0 1.0 0.0 null null null)
  (`|SpawnActorFromClass` "/Game/BluePrints/PickUps/Goop.Goop_C" (`KismetMathLibrary.MakeTransform` (`self.K2_GetActorLocation`)) "Undefined" "OverrideRootScale" null null)
  (`self.K2_DestroyActor`))

(event `self.PlayerDetection.OnComponentBeginOverlap`
  (params (OverlappedComponent :type "PrimitiveComponent Object Reference") (OtherActor :type "Actor Object Reference") (OtherComp :type "PrimitiveComponent Object Reference") (OtherBodyIndex :type Integer) (bFromSweep :type Boolean) (SweepResult :type "HitResult Structure (by ref)"))
  (bind _astest_pawn (cast `/Game/BluePrints/Units/TestPawn` OtherActor))
  (if (!= (`GameplayStatics.GetObjectClass` _astest_pawn) "/Game/BluePrints/Units/FighterSlime.FighterSlime_C")
    (`KismetArrayLibrary.Array_AddUnique` (`self.TargetPlayers`) OtherActor)
    (if (> (`KismetArrayLibrary.Array_Length` (`self.TargetPlayers`)) 0) :!label _label_7
      (`AIController.MoveToActor` (`AIBlueprintHelperLibrary.GetAIController` self) (`|GetArrayItem` (`self.TargetPlayers`)) 35.0 true true true null true)
      (else
        (goto _label_5)))))

(event `self.PlayerDetection.OnComponentEndOverlap`
  (params (OverlappedComponent :type "PrimitiveComponent Object Reference") (OtherActor :type "Actor Object Reference") (OtherComp :type "PrimitiveComponent Object Reference") (OtherBodyIndex :type Integer))
  (bind _astest_pawn (cast `/Game/BluePrints/Units/TestPawn` OtherActor))
  (if (!= (`GameplayStatics.GetObjectClass` _astest_pawn) "/Game/BluePrints/Units/FighterSlime.FighterSlime_C")
    (`KismetArrayLibrary.Array_RemoveItem` (`self.TargetPlayers`) OtherActor)
    (goto _label_7)))

(fn `UserConstructionScript`)