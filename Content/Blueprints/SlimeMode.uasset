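; SlimeMode is the game mode for a slime game with Fighter, Builder and Scavenger pawns, ending when the Queen Slime dies.
; BeginPlay builds the HUD and tutorial, binds the loss event and adds players from the options string.
; ChangeFocus re-possesses pawns for one player or toggles active controllers for three.
; It also manages three Goop currencies, tutorial pausing, and the analytics-fed end screen with restart.
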(event `Game Lost`
  (bind _returnvalue (`|CreateWidget` "/Game/Blueprints/UI/EndGameScreen.EndGameScreen_C"))
  (bind _outactors (`GameplayStatics.GetAllActorsOfClass` "/Game/Blueprints/AnalyticsManager.AnalyticsManager_C"))
  (bind _output (`|GetArrayItem` _outactors))
  (`/Game/Blueprints/AnalyticsManager.Save Round Data` _output)
  (bind _out_data (`/Game/Blueprints/AnalyticsManager.Get Total Game Data` _output))
  (`/Game/Blueprints/UI/EndGameScreen.Update Stats` _returnvalue _out_data)
  (`UserWidget.AddToViewport` _returnvalue 0)
  (`self.On Game Finished`))

(event `self.ReceiveBeginPlay`
  (bind _optionsstring (`self.OptionsString`))
  (`KismetSystemLibrary.ExecuteConsoleCommand` "EnableAllScreenMessages" null)
  (`KismetSystemLibrary.PrintString` "Hello")
  (`|ExecutionSequence`
    (:`then_0`
      (`self.PopulatePawnArray`)
      (`/Game/Blueprints/Components/TetrisRandomizer.SetArraySize` (`self.SetActiveRandomizer`) (`KismetArrayLibrary.Array_Length` (`self.PlayerActivateSounds`)))
      (bind _returnvalue (`|CreateWidget` "/Game/Blueprints/UI/SlimeHUD.SlimeHUD_C"))
      (`UserWidget.AddToViewport` _returnvalue 0)
      (set `self.HUD` _returnvalue)
      (`self.ChangeFocus` 0)
      (bind _outactors (`GameplayStatics.GetAllActorsOfClass` "/Game/Blueprints/Units/QueenSlime.QueenSlime_C"))
      (bind _output (`|GetArrayItem` _outactors))
      (`/Engine/EditorBlueprintResources/StandardMacros.IsValid` _output
        (:`Is Valid`
          (add `/Game/Blueprints/Components/Health.OnKilled` (`/Game/Blueprints/Units/Unit.Health` _output) (delegate `Game Lost`)))))
    (:`then_1`
      (if (`KismetStringLibrary.EqualEqual_StrStr` _optionsstring "?1")
        (`self.AddPlayer`)
        (elif (`KismetStringLibrary.EqualEqual_StrStr` _optionsstring "?2")
          (`self.AddPlayer`)
          (`self.AddPlayer`)
          (elif (`KismetStringLibrary.EqualEqual_StrStr` _optionsstring "?3")
            (`self.AddPlayer`)
            (`self.AddPlayer`)
            (`self.AddPlayer`)))))
    (:`then_2`
      (bind _asslime_player_controller (cast `/Game/Blueprints/SlimePlayerController` (`GameplayStatics.GetPlayerController` 0)))
      (set `/Game/Blueprints/SlimePlayerController.Active` true _asslime_player_controller))
    (:`then_3`
      (bind _returnvalue_2 (`|CreateWidget` "/Game/Blueprints/UI/TutorialWidget.TutorialWidget_C"))
      (bind _output_get (set `self.Tutorial Widget` _returnvalue_2))
      (`UserWidget.AddToViewport` _output_get 1)
      (`UserWidget.PlayAnimation` _returnvalue_2 (`/Game/Blueprints/UI/TutorialWidget.PopIn` _returnvalue_2) 0.0 1 "Forward" 1.0)
      (`Widget.SetVisibility` (`self.Tutorial Widget`) "Hidden")
      (bind _returnvalue_3 (`GameplayStatics.GetCurrentLevelName` true))
      (if (`KismetStringLibrary.EqualEqual_StrStr` _returnvalue_3 "DamenMap")
        (`KismetSystemLibrary.Delay` 1.5)
        (if (not (`Widget.IsVisible` (`self.Tutorial Widget`)))
          (`self.Toggle Tutorial Widget`))))))

(event `Restart Game`
  (bind _hud (`self.HUD`))
  (bind _fadeout (`/Game/Blueprints/UI/SlimeHUD.FadeOut` _hud))
  (`UserWidget.BindToAnimationEvent` _hud _fadeout (delegate `Loss Fade Finished`) "Finished" "None")
  (`UserWidget.PlayAnimation` _hud _fadeout 0.0 1 "Forward" 1.0))

(event `Loss Fade Finished`
  (`GameplayStatics.OpenLevel` "JoshMap"))

(event `Toggle Tutorial Widget`
  (bind _tutorial_widget (`self.Tutorial Widget`))
  (bind _tutorial_widget_2 (`self.Tutorial Widget`))
  (bind _foundwidgets (`WidgetBlueprintLibrary.GetAllWidgetsOfClass` "/Game/Blueprints/UI/EndGameScreen.EndGameScreen_C"))
  (if (> (`KismetArrayLibrary.Array_Length` _foundwidgets) 0)
    (`self.Restart Game`)
    (elif (`Widget.IsVisible` (`self.Tutorial Widget`))
      (`UserWidget.PlayAnimation` _tutorial_widget_2 (`/Game/Blueprints/UI/TutorialWidget.PopIn` _tutorial_widget_2) 0.0 1 "Reverse" 1.0)
      (`GameplayStatics.SetGamePaused` false)
      (`KismetSystemLibrary.Delay` 0.3)
      (`Widget.SetVisibility` (`self.Tutorial Widget`) "Hidden")
      (set `self.TutorialWidgetVisible` false)
      (else
        (`Widget.SetVisibility` _tutorial_widget "Visible")
        (`UserWidget.PlayAnimation` _tutorial_widget (`/Game/Blueprints/UI/TutorialWidget.PopIn` _tutorial_widget) 0.0 1 "Forward" 1.0)
        (`GameplayStatics.SetGamePaused` true)
        (set `self.TutorialWidgetVisible` true)
        (`self.Game Paused`)))))

(fn `AddExplosiveGoop`
  (params (Amount :type Integer) (`Show Popup` :type Boolean :default true) (`Instigating Actor` :type "Actor Object Reference"))
  (`/Game/Blueprints/Libraries/HelperFunctions.+=` (`self.ExplosiveGoop`) Amount)
  (`|ExecutionSequence`
    (:`then_0`
      (if (`local.Show Popup`)
        (`|SpawnActorFromClass` "/Game/Blueprints/UI/CostWidgetActor.CostWidgetActor_C" (`KismetMathLibrary.MakeTransform` (`self.K2_GetActorLocation` (`local.Instigating Actor`))) "Undefined" "OverrideRootScale" null (`local.Amount`) "NewEnumerator1" "+" null)))
    (:`then_1`
      (`self.ExplosiveGoopGained` Amount (`self.ExplosiveGoop`)))))

(fn `AddGoop`
  (params (Amount :type Integer) (`Show Popup` :type Boolean :default true) (`Instigating Actor` :type "Actor Object Reference"))
  (`/Game/Blueprints/Libraries/HelperFunctions.+=` (`self.Goop`) Amount)
  (`|ExecutionSequence`
    (:`then_0`
      (if (`local.Show Popup`)
        (`|SpawnActorFromClass` "/Game/Blueprints/UI/CostWidgetActor.CostWidgetActor_C" (`KismetMathLibrary.MakeTransform` (`self.K2_GetActorLocation` (`local.Instigating Actor`))) "Undefined" "OverrideRootScale" null (`local.Amount`) "NewEnumerator0" "+" null)))
    (:`then_1`
      (`self.GoopGained` Amount (`self.Goop`)))))

(fn `AddPlayer`
  (bind _numplayers (`self.NumPlayers`))
  (`/Engine/EditorBlueprintResources/StandardMacros.IncrementInt` (`self.NumPlayers`)
    (:`  `
      (if (== _numplayers 1)
        (bind _asslime_player_controller (cast `/Game/Blueprints/SlimePlayerController` (`GameplayStatics.GetPlayerController` 0)))
        (set `/Game/Blueprints/SlimePlayerController.JoinedGame` true _asslime_player_controller)
        (elif (== _numplayers 3)
          (bind _outactors (`GameplayStatics.GetAllActorsOfClass` "/Game/Blueprints/SlimePlayerController.SlimePlayerController_C"))
          (for _array_element _outactors
            (set `/Game/Blueprints/SlimePlayerController.JoinedGame` true _array_element)))))))

(fn `AddStickyGoop`
  (params (Amount :type Integer) (ShowPopup :type Boolean :default true) (`Instigating Actor` :type "Actor Object Reference"))
  (`/Game/Blueprints/Libraries/HelperFunctions.+=` (`self.StickyGoop`) Amount)
  (`|ExecutionSequence`
    (:`then_0`
      (if (`local.ShowPopup`)
        (`|SpawnActorFromClass` "/Game/Blueprints/UI/CostWidgetActor.CostWidgetActor_C" (`KismetMathLibrary.MakeTransform` (`self.K2_GetActorLocation` (`local.Instigating Actor`))) "Undefined" "OverrideRootScale" null (`local.Amount`) "NewEnumerator1" "+" null)))
    (:`then_1`
      (`self.StickyGoopGained` Amount (`self.StickyGoop`)))))

(fn `ChangeFocus`
  (params (Direction :type Integer))
  (bind _output (`|GetArrayItem` (`self.PawnReferences`) (`self.PossessedChar`)))
  (bind _returnvalue (mod (+ Direction (`self.PossessedChar`)) 3))
  (bind _returnvalue_2 (`Pawn.GetController` _output))
  (if (> Direction 0)
    (`/Game/Blueprints/UI/SlimeHUD.RBPressed` (`self.HUD`))
    (elif (< Direction 0)
      (`/Game/Blueprints/UI/SlimeHUD.LBPressed` (`self.HUD`))))
  (if (< _returnvalue 0)
    (set `self.PossessedChar` 2)
    (else
      (set `self.PossessedChar` _returnvalue)))
  (`/Game/Blueprints/UI/SlimeHUD.MoveFocus` (`self.HUD`) (`self.PossessedChar`))
  (`self.ShowAndHideCosts`)
  (switch `int` (`self.NumPlayers`)
    (:`1`
      (`Controller.UnPossess` (`GameplayStatics.GetPlayerController` 0))
      (if (`KismetSystemLibrary.IsValid` _output)
        (`/Game/Blueprints/Units/TestPawn.SwitchedTo` _output)
        (if (`KismetSystemLibrary.IsValid` _returnvalue_2)
          (bind _asplayer_controller (cast `PlayerController` _returnvalue_2)
            (:`then`
              (`Controller.UnPossess` _asplayer_controller))
            (:`CastFailed`
              _)))
        (`Controller.Possess` (`GameplayStatics.GetPlayerController` 0) _output)
        (bind _index (`/Game/Blueprints/Components/TetrisRandomizer.PickIndex` (`self.SetActiveRandomizer`)))
        (`GameplayStatics.PlaySoundAtLocation` (`|GetArrayItem` (`self.PlayerActivateSounds`) _index) (`self.K2_GetActorLocation` _output) (struct) 1.0 1.0 0.0 null null null)
        (`self.ControlSwitched` _output)))
    (:`3`
      (for _array_element (`self.PawnReferences`)
        (bind _asslime_player_controller (cast `/Game/Blueprints/SlimePlayerController` (`Pawn.GetController` _array_element)))
        (if (== (`GameplayStatics.GetPlayerControllerID` _asslime_player_controller) (`self.PossessedChar`))
          (set `/Game/Blueprints/SlimePlayerController.Active` true _asslime_player_controller)
          (bind _index_2 (`/Game/Blueprints/Components/TetrisRandomizer.PickIndex` (`self.SetActiveRandomizer`)))
          (bind _returnvalue_3 (`Controller.K2_GetPawn` _asslime_player_controller))
          (`GameplayStatics.PlaySoundAtLocation` (`|GetArrayItem` (`self.PlayerActivateSounds`) _index_2) (`self.K2_GetActorLocation` _returnvalue_3) (struct) 1.0 1.0 0.0 null null null)
          (bind _astest_pawn (cast `/Game/Blueprints/Units/TestPawn` _returnvalue_3))
          (`/Game/Blueprints/Units/TestPawn.SwitchedTo` _astest_pawn)
          (`self.ControlSwitched` _astest_pawn)
          (else
            (set `/Game/Blueprints/SlimePlayerController.Active` false _asslime_player_controller)))))))

(fn `MakeExplosiveGoop`
  (returns (Success :type Boolean))
  (if (<= (`self.Goop`) 0)
    (return false)
    (else
      (`/Game/Blueprints/Libraries/HelperFunctions.+=` (`self.Goop`) -1)
      (`/Game/Blueprints/Libraries/HelperFunctions.+=` (`self.ExplosiveGoop`) 2)
      (`KismetSystemLibrary.PrintString` "I have a bad case of explosive Goop")
      (return true))))

(fn `MakeStickyGoop`
  (returns (Success :type Boolean))
  (if (<= (`self.Goop`) 0)
    (return false)
    (else
      (`/Game/Blueprints/Libraries/HelperFunctions.+=` (`self.Goop`) -1)
      (`/Game/Blueprints/Libraries/HelperFunctions.+=` (`self.StickyGoop`) 4)
      (`KismetSystemLibrary.PrintString` "What's this sticky Goop?")
      (return true))))

(fn `PopulatePawnArray`
  (bind _outactors (`GameplayStatics.GetAllActorsOfClass` "/Game/Blueprints/Units/FighterSlime.FighterSlime_C"))
  (`KismetArrayLibrary.Array_Set` (`self.PawnReferences`) 0 (`|GetArrayItem` _outactors))
  (bind _outactors_2 (`GameplayStatics.GetAllActorsOfClass` "/Game/Blueprints/Units/BuilderSlime.BuilderSlime_C"))
  (`KismetArrayLibrary.Array_Set` (`self.PawnReferences`) 1 (`|GetArrayItem` _outactors_2))
  (bind _outactors_3 (`GameplayStatics.GetAllActorsOfClass` "/Game/Blueprints/Units/ScavengerSlime.ScavengerSlime_C"))
  (`KismetArrayLibrary.Array_Set` (`self.PawnReferences`) 2 (`|GetArrayItem` _outactors_3)))

(fn `ShowAndHideCosts`
  (bind _outactors (`GameplayStatics.GetAllActorsOfClass` "/Game/Blueprints/Structures/Interactable/StationParentClass.StationParentClass_C"))
  (for _array_element _outactors
    (`/Game/Blueprints/Structures/Interactable/StationParentClass.HideCostWidget` _array_element)
    (`/Game/Blueprints/Structures/Interactable/StationParentClass.ShowCostWidget` _array_element)))

(fn `UseExplosiveGoop`
  (params (Cost :type Integer))
  (returns (Success :type Boolean))
  (if (>= (`self.ExplosiveGoop`) Cost)
    (`/Game/Blueprints/Libraries/HelperFunctions.+=` (`self.ExplosiveGoop`) (* Cost -1))
    (return true)
    (else
      (return false))))

(fn `UserConstructionScript`)

(fn `UseStickyGoop`
  (params (Cost :type Integer))
  (returns (Success :type Boolean))
  (if (>= (`self.StickyGoop`) Cost)
    (`/Game/Blueprints/Libraries/HelperFunctions.+=` (`self.StickyGoop`) (* Cost -1))
    (return true)
    (else
      (return false))))