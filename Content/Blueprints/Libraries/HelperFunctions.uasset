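; Blueprint helper library with a by-reference add-assign utility and a nearest-actor search.
; The += graph writes a variable plus an amount back into that variable.
; GetClosestActorToActors loops over candidates, keeping the one whose distance to the source beats DistanceOfClosest, and returns nothing if the first is invalid.
; ClosestSoFar starts as the first candidate, but DistanceOfClosest is not seeded from that candidate's distance.
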(fn `+=`
  (params (Variable :type "Integer (by ref)") (Amount :type Integer))
  (`|VariableSetRef` Variable (+ Variable Amount)))

(fn `GetClosestActorToActors`
  (params (`Source Actor` :type "Actor Object Reference") (`Candidate Actors` :type "Array of Actor Object Reference"))
  (returns (`Closest Actor` :type "Actor Object Reference"))
  (locals (`Closest So Far` :type "Actor Object Reference") (`Distance of Closest` :type "Float (double-precision)" :default 999999.0))
  (bind _output (`|GetArrayItem` `Candidate Actors`))
  (`/Engine/EditorBlueprintResources/StandardMacros.IsValid` _output
    (:`Is Valid`
      (set `local.Closest So Far` _output)
      (for _array_element `Candidate Actors`
        (bind _returnvalue (`KismetMathLibrary.VSize` (- (`Actor.K2_GetActorLocation` _array_element) (`Actor.K2_GetActorLocation` `Source Actor`))))
        (if (< _returnvalue (`local.Distance of Closest`))
          (set `local.Closest So Far` _array_element)
          (set `local.Distance of Closest` _returnvalue)))
      (return (`local.Closest So Far`)))
    (:`Is Not Valid`
      (return null))))