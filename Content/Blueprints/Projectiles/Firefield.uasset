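; Firefield is a projectile-folder Blueprint that sets off a spreading field of fire, triggered by its Fire event or the 7 key.
; Fire deals heavy one-time damage to the Health component of every Slime overlapping its Box and activates the center particle systems at once.
; It then activates matching left and right particle pairs outward in five steps with random delays between them, so only the visuals spread over time.
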(event `Key|Seven`
  (params (Key :type "Key Structure"))
  (:`Pressed`
    (`self.Fire`)))

(event `Fire`
  (bind _returnvalue (`KismetMathLibrary.RandomFloatInRange` (`self.Minimum Delay`) (`self.Maximum Delay`)))
  (`|ExecutionSequence`
    (:`then_0`
      (for _array_element (`PrimitiveComponent.GetOverlappingActors` (`self.Box`) "/Game/Blueprints/Units/Slime.Slime_C")
        (`/Game/Blueprints/Health.Damage` (`self.GetComponentByClass` _array_element "/Game/Blueprints/Health.Health_C") 2000.0))
      (for _array_element_2 (`self.Center Pieces`)
        (`ActorComponent.Activate` _array_element_2 false)))
    (:`then_1`
      (`KismetSystemLibrary.Delay` _returnvalue)
      (`self.Propogate Fire` 0)
      (`KismetSystemLibrary.Delay` _returnvalue)
      (`self.Propogate Fire` 1)
      (`KismetSystemLibrary.Delay` _returnvalue)
      (`self.Propogate Fire` 2)
      (`KismetSystemLibrary.Delay` _returnvalue)
      (`self.Propogate Fire` 3)
      (`KismetSystemLibrary.Delay` _returnvalue)
      (`self.Propogate Fire` 4))))

(event `Propogate Fire`
  (params (Index :type Integer))
  (`ActorComponent.Activate` (`|GetArrayItem` (`self.Left Pieces`) Index) false)
  (`ActorComponent.Activate` (`|GetArrayItem` (`self.Right Pieces`) Index) false))

(event `self.ReceiveBeginPlay`
  (set `self.Center Pieces` (`|MakeArray` (`self.ParticleSystem_R1`) (`self.ParticleSystem_Center`) (`self.ParticleSystem_L1`)))
  (set `self.Right Pieces` (`|MakeArray` (`self.ParticleSystem_R2`) (`self.ParticleSystem_R3`) (`self.ParticleSystem_R4`) (`self.ParticleSystem_R5`) (`self.ParticleSystem_R6`)))
  (set `self.Left Pieces` (`|MakeArray` (`self.ParticleSystem_L2`) (`self.ParticleSystem_L3`) (`self.ParticleSystem_L4`) (`self.ParticleSystem_L5`) (`self.ParticleSystem_L6`))))

(fn `UserConstructionScript`)