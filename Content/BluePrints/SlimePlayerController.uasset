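; Player controller for a slime game: Cancel joins through SlimeMode, then input drives movement, aim and TestPawn interactions.
; Only an Active controller moves, interacts or passes focus through SlimeMode.ChangeFocus.
; When inactive, interact and cancel play an "oops" failure, while focus buttons show an attention widget and sound.
; Attention volume drops with each call and recovers on a looping timer, damping spam.
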(event `InputAction|Cancel`
  (params (Key :type "Key Structure"))
  (:`Pressed`
    (if (not (`self.JoinedGame`))
      (`self.JoinGame`))))

(event `JoinGame`
  (set `self.JoinedGame` true)
  (bind _asslime_mode (cast `/Game/Blueprints/SlimeMode` (`GameplayStatics.GetGameMode`)))
  (`/Game/Blueprints/SlimeMode.AddPlayer` _asslime_mode))

(event `self.ReceiveBeginPlay`
  (`/Game/Blueprints/Components/TetrisRandomizer.SetArraySize` (`self.AttentionSoundRandomizer`) (`KismetArrayLibrary.Array_Length` (`self.AttentionSounds`)))
  (`/Game/Blueprints/Components/TetrisRandomizer.SetArraySize` (`self.OopsSoundRandomizer`) (`KismetArrayLibrary.Array_Length` (`self.OopsSounds`)))
  (`KismetSystemLibrary.K2_SetTimerDelegate` (delegate `IncreaseAttentionVolume`) 0.05 true))

(event `self.ReceiveTick`
  (params (DeltaSeconds :type "Float (single-precision)"))
  (bind _astest_pawn (cast `/Game/Blueprints/Units/TestPawn` (`self.K2_GetPawn`)))
  (set `self.SpeedModifier` (`/Game/Blueprints/Units/TestPawn.SpeedModifier` _astest_pawn)))

(event `IncreaseAttentionVolume`
  (set `self.AttentionVolume` (`KismetMathLibrary.FMin` (+ (`self.AttentionVolume`) 0.01) (`self.MaxAttentionVolume`))))

(event `InputAxis|MoveRight`
  (params (AxisValue :type "Float (single-precision)"))
  (bind _returnvalue (`self.K2_GetPawn`))
  (if (`self.JoinedGame`)
    (if (`self.Active`)
      (if (`KismetSystemLibrary.IsValid` _returnvalue)
        (`Pawn.AddMovementInput` _returnvalue (`KismetMathLibrary.MakeVector` 0.0 AxisValue) (`self.SpeedModifier`) false)))))

(event `InputAxis|MoveUp`
  (params (AxisValue :type "Float (single-precision)"))
  (bind _returnvalue (`self.K2_GetPawn`))
  (if (`self.JoinedGame`)
    (if (`self.Active`)
      (if (`KismetSystemLibrary.IsValid` _returnvalue)
        (`Pawn.AddMovementInput` _returnvalue (`KismetMathLibrary.MakeVector` AxisValue) (`self.SpeedModifier`) false)))))

(event `InputAction|Interact`
  (params (Key :type "Key Structure"))
  (bind _returnvalue (`self.K2_GetPawn`))
  (bind _active (`self.Active`))
  (bind _joinedgame (`self.JoinedGame`))
  (:`Pressed`
    (if _joinedgame
      (if _active
        (bind _astest_pawn (cast `/Game/Blueprints/Units/TestPawn` _returnvalue))
        (`/Game/Blueprints/Units/TestPawn.TryInteract` _astest_pawn)
        (else
          (`self.Oops`)))))
  (:`Released`
    (if _joinedgame
      (if _active
        (bind _astest_pawn_2 (cast `/Game/Blueprints/Units/TestPawn` _returnvalue))
        (`/Game/Blueprints/Units/TestPawn.TryRelease` _astest_pawn_2)))))

(event `InputAction|Cancel`
  (params (Key :type "Key Structure"))
  (:`Released`
    (if (`self.JoinedGame`)
      (if (`self.Active`)
        (bind _astest_pawn (cast `/Game/Blueprints/Units/TestPawn` (`self.K2_GetPawn`)))
        (`/Game/Blueprints/Units/TestPawn.TryCancel` _astest_pawn)
        (else
          (`self.Oops`))))))

(event `InputAction|FocusLeft`
  (params (Key :type "Key Structure"))
  (:`Pressed`
    (if (`self.JoinedGame`)
      (if (`self.Active`)
        (bind _astest_pawn (cast `/Game/Blueprints/Units/TestPawn` (`self.K2_GetPawn`)))
        (`/Game/Blueprints/Units/TestPawn.ISwitched` _astest_pawn)
        (bind _asslime_mode (cast `/Game/Blueprints/SlimeMode` (`GameplayStatics.GetGameMode`)))
        (`/Game/Blueprints/SlimeMode.ChangeFocus` _asslime_mode -1)
        (else
          (`self.AttentionPls`))))))

(event `InputAction|FocusRight`
  (params (Key :type "Key Structure"))
  (:`Pressed`
    (if (`self.JoinedGame`)
      (if (`self.Active`)
        (bind _astest_pawn (cast `/Game/Blueprints/Units/TestPawn` (`self.K2_GetPawn`)))
        (`/Game/Blueprints/Units/TestPawn.ISwitched` _astest_pawn)
        (bind _asslime_mode (cast `/Game/Blueprints/SlimeMode` (`GameplayStatics.GetGameMode`)))
        (`/Game/Blueprints/SlimeMode.ChangeFocus` _asslime_mode 1)
        (else
          (`self.AttentionPls`))))))

(event `InputAxis|AimRight`
  (params (AxisValue :type "Float (single-precision)"))
  (if (`self.JoinedGame`)
    (set `self.AimDirection` (`KismetMathLibrary.MakeVector` (.x (`self.AimDirection`)) AxisValue (.z (`self.AimDirection`))))))

(event `InputAxis|AimUp`
  (params (AxisValue :type "Float (single-precision)"))
  (if (`self.JoinedGame`)
    (set `self.AimDirection` (`KismetMathLibrary.MakeVector` AxisValue (.y (`self.AimDirection`)) (.z (`self.AimDirection`))))))

(fn `AttentionPls`
  (bind _returnvalue (`self.K2_GetPawn`))
  (bind _returnvalue_2 (`|CreateWidget` "/Game/Blueprints/UI/AttentionWidget.AttentionWidget_C" null _returnvalue))
  (`UserWidget.AddToViewport` _returnvalue_2 0)
  (bind _index (`/Game/Blueprints/Components/TetrisRandomizer.PickIndex` (`self.AttentionSoundRandomizer`)))
  (`GameplayStatics.PlaySoundAtLocation` (`|GetArrayItem` (`self.AttentionSounds`) _index) (`self.K2_GetActorLocation` _returnvalue) (struct) (`self.AttentionVolume`) 1.0 0.0 null null null)
  (set `self.AttentionVolume` (`KismetMathLibrary.FMax` (- (`self.AttentionVolume`) 0.1) (`self.MinAttentionVolume`))))

(fn `Oops`
  (bind _astest_pawn (cast `/Game/Blueprints/Units/TestPawn` (`self.K2_GetPawn`)))
  (`/Game/Blueprints/Units/TestPawn.InputFailed` _astest_pawn)
  (bind _index (`/Game/Blueprints/Components/TetrisRandomizer.PickIndex` (`self.OopsSoundRandomizer`)))
  (`GameplayStatics.PlaySoundAtLocation` (`|GetArrayItem` (`self.OopsSounds`) _index) (`self.K2_GetActorLocation` (`self.K2_GetPawn`)) (struct) 0.6 1.0 0.0 null null null))

(fn `UserConstructionScript`)