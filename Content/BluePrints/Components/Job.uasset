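; Job component that tracks a timed task through begin, finish and cancel events, each firing its own dispatcher.
; Begin records the start time, sets InProgress and, with AutoFinish on, calls Finish after a Delay of ExecutionTime.
; Cancel clears InProgress but leaves a pending Delay running, so Finish can still fire afterwards.
; GetCurrentTime returns elapsed seconds, or zero once ExecutionTime is exceeded.
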(event `Begin`
  (set `self.StartTime` (`KismetSystemLibrary.GetGameTimeInSeconds`))
  (set `self.InProgress` true)
  (`self.OnBegin`)
  (if (`self.AutoFinish`)
    (`KismetSystemLibrary.Delay` (`self.ExecutionTime`))
    (`self.Finish`)))

(event `Finish`
  (set `self.InProgress` false)
  (`self.OnFinish`))

(event `Cancel`
  (set `self.InProgress` false)
  (`self.OnCancel`))

(fn `GetCurrentTime`
  (returns (CurrentTIme :type "Float (double-precision)"))
  (bind _returnvalue (- (`KismetSystemLibrary.GetGameTimeInSeconds`) (`self.StartTime`)))
  (if (> _returnvalue (`self.ExecutionTime`))
    (return 0.0)
    (else
      (return _returnvalue))))