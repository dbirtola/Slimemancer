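; Health component that tracks current health and reports damage, healing and death through event dispatchers.
; Damage subtracts from Health without clamping, calls OnDamaged, then fires Death whenever the result is zero or below, which calls OnKilled.
; Heal adds to Health capped at MaxHealth and calls OnHealed.
; No guard prevents Death from firing again on further damage.
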(event `Death`
  (`self.OnKilled`))

(fn `Damage`
  (params (Amount :type "Float (double-precision)"))
  (set `self.Health` (- (`self.Health`) Amount))
  (`self.OnDamaged` (`local.Amount`))
  (if (<= (`self.Health`) 0.0)
    (`self.Death`)))

(fn `Heal`
  (params (Amount :type "Float (double-precision)"))
  (set `self.Health` (`KismetMathLibrary.FMin` (+ (`self.Health`) Amount) (`self.MaxHealth`)))
  (`self.OnHealed` (`local.Amount`)))