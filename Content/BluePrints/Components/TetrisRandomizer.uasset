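; TetrisRandomizer is a shuffle-bag randomizer that hands out indices in random order, in the style of Tetris piece selection.
; SetArraySize fills an array with indices from zero to Size minus one, calling Randomize after each addition to shuffle and reset the cursor.
; PickIndex advances the cursor before reading, so the first pick after setup skips slot zero, and reshuffles once the bag runs out.
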(event `SetArraySize`
  (params (Size :type Integer))
  (bind _output_get (set `self.Size` Size))
  (`KismetArrayLibrary.Array_Clear` (`self.IntArray`))
  (for _index (range _output_get)
    (`KismetArrayLibrary.Array_AddUnique` (`self.IntArray`) _index)
    (`self.Randomize`)))

(fn `PickIndex`
  (returns (Index :type Integer))
  (`/Engine/EditorBlueprintResources/StandardMacros.IncrementInt` (`self.CurrentIndex`)
    (:`  `
      (if (not (< (`self.CurrentIndex`) (`self.Size`)))
        (`self.Randomize`))
      (return (`|GetArrayItem` (`self.IntArray`) (`self.CurrentIndex`))))))

(fn `Randomize`
  (`KismetArrayLibrary.Array_Shuffle` (`self.IntArray`))
  (set `self.CurrentIndex` 0))