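; TestPawn is a test pawn that sends interaction messages to actors overlapping its box and can receive them itself.
; TryInteract and TryRelease loop over the Box component's overlapping actors and send each an InteractPressed or InteractReleased interface message.
; Its own InteractPressed event only prints a debug string, and nothing in this Blueprint calls either function.
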(event `/Game/BluePrints/Interfaces/Interactable.InteractPressed`
  (`KismetSystemLibrary.PrintString` "Interacting!"))

(fn `TryInteract`
  (for _array_element (`PrimitiveComponent.GetOverlappingActors` (`self.Box`) null)
    (message `/Game/BluePrints/Interfaces/Interactable.InteractPressed` _array_element)))

(fn `TryRelease`
  (for _array_element (`PrimitiveComponent.GetOverlappingActors` (`self.Box`) null)
    (message `/Game/BluePrints/Interfaces/Interactable.InteractReleased` _array_element)))

(fn `UserConstructionScript`)