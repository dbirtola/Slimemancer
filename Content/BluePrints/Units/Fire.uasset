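; Fire hazard actor that repeatedly burns units of one specific faction standing inside its sphere.
; It records its spawn time and deals no damage until a short hard-coded warm-up has passed.
; Tick runs through a DoOnce reset after an AttackCooldown delay, so each pulse applies FlameDamage to overlapping actors whose Health component matches that faction.
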(event `self.ReceiveBeginPlay`
  (set `self.StartTime` (`KismetSystemLibrary.GetGameTimeInSeconds`)))

(event `self.ReceiveTick`
  (params (DeltaSeconds :type "Float (single-precision)"))
  (`/Engine/EditorBlueprintResources/StandardMacros.DoOnce` false :!label _label
    (:`Completed`
      (if (> (- (`KismetSystemLibrary.GetGameTimeInSeconds`) (`self.StartTime`)) 1.3)
        (for _array_element (`PrimitiveComponent.GetOverlappingActors` (`self.Sphere`) "/Script/Engine.Actor")
          (bind _returnvalue (`self.GetComponentByClass` _array_element "/Game/Blueprints/Components/Health.Health_C"))
          (`/Engine/EditorBlueprintResources/StandardMacros.IsValid` _returnvalue
            (:`Is Valid`
              (if (`|EnumEquality` (`/Game/Blueprints/Components/Health.Faction` _returnvalue) "NewEnumerator0")
                (`/Game/Blueprints/Components/Health.Damage` _returnvalue (`self.FlameDamage`)))))))
      (`KismetSystemLibrary.Delay` (`self.AttackCooldown`))
      (goto _label :!via `Reset`))))

(fn `UserConstructionScript`)