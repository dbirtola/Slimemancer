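; Meteor projectile actor that travels from its spawn point to a Target location and leaves fire on impact.
; Tick linearly interpolates its position by elapsed game time over Time, using a swept move with a set Rotation.
; On arrival it spawns an impact particle and an enlarged Fire actor with random pitch, then destroys itself.
; The sphere's overlap and hit events are empty, so impact depends only on timing.
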(event `self.ReceiveBeginPlay`
  (set `self.StartTime` (`KismetSystemLibrary.GetGameTimeInSeconds`))
  (set `self.Start` (`self.K2_GetActorLocation` self)))

(event `self.ReceiveTick`
  (params (DeltaSeconds :type "Float (single-precision)"))
  (bind _target (`self.Target`))
  (bind _returnvalue (`KismetMathLibrary.FMin` (/ (- (`KismetSystemLibrary.GetGameTimeInSeconds`) (`self.StartTime`)) (`self.Time`)) 1.0))
  (`self.K2_SetActorLocationAndRotation` (`KismetMathLibrary.VLerp` (`self.Start`) (`self.Target`) _returnvalue) (`self.Rotation`) true)
  (if (== _returnvalue 1.0)
    (`GameplayStatics.SpawnEmitterAtLocation` "/Game/ParticleSystems/P_ProjectileImpact.P_ProjectileImpact" _target)
    (`|SpawnActorFromClass` "/Game/BluePrints/Units/Fire.Fire_C" (`KismetMathLibrary.MakeTransform` _target (`KismetMathLibrary.MakeRotator` 0.0 (`KismetMathLibrary.RandomFloatInRange` 0.0 360.0)) (4.0 4.0 4.0)) "Undefined" "OverrideRootScale" null null)
    (`self.K2_DestroyActor`)))

(event `self.Sphere.OnComponentBeginOverlap`
  (params (OverlappedComponent :type "PrimitiveComponent Object Reference") (OtherActor :type "Actor Object Reference") (OtherComp :type "PrimitiveComponent Object Reference") (OtherBodyIndex :type Integer) (bFromSweep :type Boolean) (SweepResult :type "HitResult Structure (by ref)")))

(event `self.Sphere.OnComponentHit`
  (params (HitComponent :type "PrimitiveComponent Object Reference") (OtherActor :type "Actor Object Reference") (OtherComp :type "PrimitiveComponent Object Reference") (NormalImpulse :type "Vector Structure") (Hit :type "HitResult Structure (by ref)")))

(fn `UserConstructionScript`)