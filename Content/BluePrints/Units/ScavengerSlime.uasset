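; Scavenger slime unit that launches itself through the air to a player-aimed landing point.
; Holding interact freezes movement and steers an indicator actor by the controller's aim direction, clamped to Range.
; Releasing starts a timed Job shown on a progress bar while Tick moves the slime along a lerp with a sine-based height arc.
; On arrival it destroys the indicator, restores the speed modifier and finishes the Job.
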(event `self.ReceiveBeginPlay`
  (set `/Game/Blueprints/Components/Job.ExecutionTime` (`self.TravelTime`) (`self.Job`))
  (bind _asjob_progres (cast `/Game/Blueprints/UI/JobProgres` (`WidgetComponent.GetUserWidgetObject` (`self.JobProgressBar`))))
  (`/Game/Blueprints/UI/JobProgres.Bind To Job` _asjob_progres (`self.Job`)))

(event `self.ReceiveTick`
  (params (DeltaSeconds :type "Float (single-precision)"))
  (if (`self.Held`)
    (`self.MoveIndicator`))
  (if (>= (`self.TimeTravelled`) 0.0)
    (set `self.TimeTravelled` (`KismetMathLibrary.FClamp` (+ DeltaSeconds (`self.TimeTravelled`)) 0.0 (`self.TravelTime`)))
    (`self.CalculateNewLocation`)
    (if (>= (`self.TimeTravelled`) (`self.TravelTime`))
      (set `self.TimeTravelled` -1.0)
      (`self.K2_DestroyActor` (`self.Indicator`))
      (bind _asslime_player_controller (cast `/Game/Blueprints/SlimePlayerController` (`self.GetController`)))
      (set `/Game/Blueprints/SlimePlayerController.SpeedModifier` 1.0 _asslime_player_controller)
      (`/Game/Blueprints/Components/Job.Finish` (`self.Job`)))))

(event `self.TryInteract`
  (if (< (`self.TimeTravelled`) 0.0)
    (`self.ResetFiringVariables`)))

(event `self.TryRelease`
  (set `self.Held` false)
  (set `self.TimeTravelled` 0.0)
  (set `self.StartingPoint` (`self.K2_GetActorLocation`))
  (set `self.TargetPoint` (`self.K2_GetActorLocation` (`self.Indicator`)))
  (`/Game/Blueprints/Components/Job.Begin` (`self.Job`)))

(fn `CalculateNewLocation`
  (`self.K2_SetActorLocation` (`KismetMathLibrary.MakeVector` (.x (`KismetMathLibrary.VLerp` (`self.StartingPoint`) (`self.TargetPoint`) (/ (`self.TimeTravelled`) (`self.TravelTime`)))) (.y (`KismetMathLibrary.VLerp` (`self.StartingPoint`) (`self.TargetPoint`) (/ (`self.TimeTravelled`) (`self.TravelTime`)))) (+ (* (`KismetMathLibrary.Sin` (* (/ (`self.TimeTravelled`) (`self.TravelTime`)) (`KismetMathLibrary.GetPI`))) (`self.RiseFactor`)) (.z (`self.TargetPoint`)) (* (- (.z (`self.StartingPoint`)) (.z (`self.TargetPoint`))) (- 1.0 (/ (`self.TimeTravelled`) (`self.TravelTime`))))))))

(fn `MoveIndicator`
  (bind _asslime_player_controller (cast `/Game/Blueprints/SlimePlayerController` (`self.GetController`)))
  (bind _returnvalue (+ (* (`/Game/Blueprints/SlimePlayerController.AimDirection` _asslime_player_controller) 8.0) (`self.K2_GetActorLocation` (`self.Indicator`))))
  (bind _returnvalue_2 (- _returnvalue (`self.K2_GetActorLocation`)))
  (if (<= (`KismetMathLibrary.VSize` _returnvalue_2) (`self.Range`))
    (`self.K2_SetActorLocation` (`self.Indicator`) _returnvalue false false)
    (else
      (`self.K2_SetActorLocation` (`self.Indicator`) (+ (* (`KismetMathLibrary.Normal` _returnvalue_2) (`self.Range`)) (`self.K2_GetActorLocation`)) false false))))

(fn `ResetFiringVariables`
  (set `self.Held` true)
  (bind _asslime_player_controller (cast `/Game/Blueprints/SlimePlayerController` (`self.GetController`)))
  (set `/Game/Blueprints/SlimePlayerController.SpeedModifier` 0.0 _asslime_player_controller)
  (if (`KismetSystemLibrary.IsValid` (`self.Indicator`))
    (`self.K2_SetActorLocation` (`self.Indicator`) (`self.K2_GetActorLocation`) false false)
    (else
      (bind _returnvalue (`|SpawnActorFromClass` "/Game/Blueprints/Projectiles/Indicator.Indicator_C" (`self.GetTransform`) "Undefined" "OverrideRootScale" null null))
      (set `self.Indicator` _returnvalue))))

(fn `UserConstructionScript`
  (`parent.UserConstructionScript`))