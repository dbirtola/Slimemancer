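; BuilderSlime is a slime unit that sprays water to put out fires while its player controller supplies an aim direction.
; Tick calls AimExtinguisher, which, if the slime is not working and the controller is active, attaches a water emitter, plays audio and turns the slime toward the aim.
; The Cube's Z scale grows with hold time, destroying overlapping Fire actors.
; Releasing aim resets the Cube and stops the spray.
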(event `self.ReceiveTick`
  (params (DeltaSeconds :type "Float (single-precision)"))
  (bind _extemitter (`self.ExtEmitter`))
  (`parent.ReceiveTick` DeltaSeconds)
  (bind _asslime_player_controller (cast `/Game/Blueprints/SlimePlayerController` (`self.GetController`)))
  (if (> (`KismetMathLibrary.VSize` (`/Game/Blueprints/SlimePlayerController.AimDirection` _asslime_player_controller)) 0.1)
    (`self.AimExtinguisher`)
    (else
      (set `self.TimeHeld` 0.0)
      (`SceneComponent.SetRelativeScale3D` (`self.Cube`) (`KismetMathLibrary.MakeVector` 1.25 2.25 1.25))
      (`/Engine/EditorBlueprintResources/StandardMacros.IsValid` _extemitter
        (:`Is Valid`
          (`AudioComponent.FadeOut` (`self.SprayCycle`) 0.1 0.0)
          (`ActorComponent.K2_DestroyComponent` _extemitter))))))

(event `self.ExtPart.OnSystemFinished`
  (params (PSystem :type "ParticleSystemComponent Object Reference"))
  (`KismetSystemLibrary.PrintString` "Hello"))

(fn `AimExtinguisher`
  (bind _returnvalue (`self.K2_GetActorLocation`))
  (bind _currentjob (`self.IsWorking`))
  (bind _asslime_player_controller (cast `/Game/Blueprints/SlimePlayerController` (`self.GetController`)))
  (if (not (or _currentjob (not (`/Game/Blueprints/SlimePlayerController.Active` _asslime_player_controller))))
    (if (not (`KismetSystemLibrary.IsValid` (`self.ExtEmitter`)))
      (bind _returnvalue_2 (`GameplayStatics.SpawnEmitterAttached` "/Game/ParticleSystems/P_WaterShoot.P_WaterShoot" (`self.CapsuleComponent`) "None" (70.0 0.0 0.0) (struct :`Yaw` -90.0)))
      (set `self.ExtEmitter` _returnvalue_2)
      (`GameplayStatics.PlaySoundAtLocation` "/Game/Sounds/voice/Im_Up/eagerVoice.eagerVoice" (`self.K2_GetActorLocation` self) (struct) 1.0 1.0 0.0 null null null)
      (`AudioComponent.FadeIn` (`self.SprayCycle`) 0.1 1.0 0.0))
    (set `self.TimeHeld` (`KismetMathLibrary.FClamp` (+ (`self.TimeHeld`) (`GameplayStatics.GetWorldDeltaSeconds`)) 0.0 (`self.ChargeTime`)))
    (bind _asslime_player_controller_2 (cast `/Game/Blueprints/SlimePlayerController` (`self.GetController`)))
    (`self.K2_SetActorRotation` (`KismetMathLibrary.FindLookAtRotation` _returnvalue (+ _returnvalue (`/Game/Blueprints/SlimePlayerController.AimDirection` _asslime_player_controller_2))))
    (`SceneComponent.SetRelativeScale3D` (`self.Cube`) (`KismetMathLibrary.MakeVector` 1.25 2.25 (`KismetMathLibrary.Lerp` 1.25 7.0 (/ (`self.TimeHeld`) (`self.ChargeTime`)))))
    (for _array_element (`PrimitiveComponent.GetOverlappingActors` (`self.Cube`) "/Game/Blueprints/Units/Fire.Fire_C")
      (`self.K2_DestroyActor` _array_element))))

(fn `UserConstructionScript`
  (`parent.UserConstructionScript`))