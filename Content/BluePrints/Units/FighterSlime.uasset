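; Player-controlled fighter slime unit that lobs a timed volley of fireballs at a movable target indicator.
; Controller aim input spawns and moves the indicator, clamped within Range of the slime.
; Interacting, when not otherwise handled by the parent, starts a progress-bar-bound Job and looping timer, each shot consuming explosive goop from SlimeMode.
; Job finish or cancel, including running out of goop, clears the timer and destroys the indicator.
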(event `self.ReceiveBeginPlay`
  (`parent.ReceiveBeginPlay`)
  (bind _asjob_progres (cast `/Game/Blueprints/UI/JobProgres` (`WidgetComponent.GetUserWidgetObject` (`self.ProgressBAr`))))
  (`/Game/Blueprints/UI/JobProgres.Bind To Job` _asjob_progres (`self.Job`))
  (set `/Game/Blueprints/Components/Job.ExecutionTime` (* (- (`self.NumFires`) 1) (`self.FireTime`)) (`self.Job`)))

(event `self.ReceiveTick`
  (params (DeltaSeconds :type "Float (single-precision)"))
  (`parent.ReceiveTick` DeltaSeconds)
  (bind _asslime_player_controller (cast `/Game/Blueprints/SlimePlayerController` (`self.GetController`)))
  (if (or (> (`KismetMathLibrary.VSize` (`/Game/Blueprints/SlimePlayerController.AimDirection` _asslime_player_controller)) 0.1) (`KismetSystemLibrary.IsValid` (`self.Indicator`)))
    (`self.MoveIndicator`)))

(event `self.TryCancel`
  (bind _indicator (`self.Indicator`))
  (`parent.TryCancel`)
  (`/Engine/EditorBlueprintResources/StandardMacros.IsValid` _indicator :!label _label
    (:`Is Valid`
      (`self.K2_DestroyActor` _indicator))))

(event `self.Job.OnCancel`
  (`KismetSystemLibrary.K2_ClearAndInvalidateTimerHandle` (`self.FireTimerHandle`) :!label _label_2)
  (goto _label))

(event `self.Job.OnFinish`
  (goto _label_2))

(fn `FireFireball`
  (bind _indicator (`self.Indicator`))
  (bind _asslime_mode (cast `/Game/Blueprints/SlimeMode` (`GameplayStatics.GetGameMode`)))
  (bind _success (`/Game/Blueprints/SlimeMode.UseExplosiveGoop` _asslime_mode 1))
  (if _success
    (if (`KismetSystemLibrary.IsValid` _indicator)
      (bind _returnvalue (`|SpawnActorFromClass` "/Game/Blueprints/Projectiles/Fireball.Fireball_C" (`self.GetTransform`) "Undefined" "OverrideRootScale" null (`self.K2_GetActorLocation` _indicator) null))
      (`GameplayStatics.SpawnSoundAtLocation` "/Game/Sounds/WetWoosh.WetWoosh" (`self.K2_GetActorLocation` _returnvalue) (struct) 1.0 1.0 0.0 null null))
    (else
      (`/Game/Blueprints/Components/Job.Cancel` (`self.Job`))
      (`self.InputFailed`))))

(fn `InteractPressed`
  (params (`Interacting Actor` :type "/Game/Blueprints/Units/TestPawn Object Reference"))
  (returns (Success :type Boolean) (Job :type "/Game/Blueprints/Components/Job Object Reference"))
  (bind _success (`parent.InteractPressed` `Interacting Actor`))
  (return _success null))

(fn `MoveIndicator`
  (`/Engine/EditorBlueprintResources/StandardMacros.IsValid` (`self.Indicator`)
    (:`Is Valid`
      _)
    (:`Is Not Valid`
      (bind _returnvalue (`|SpawnActorFromClass` "/Game/Blueprints/Projectiles/Indicator.Indicator_C" (`self.GetTransform`) "Undefined" "OverrideRootScale" null null))
      (set `self.Indicator` _returnvalue)))
  (bind _asslime_player_controller (cast `/Game/Blueprints/SlimePlayerController` (`self.GetController`)))
  (bind _returnvalue_2 (+ (* (`/Game/Blueprints/SlimePlayerController.AimDirection` _asslime_player_controller) 20.0) (`self.K2_GetActorLocation` (`self.Indicator`))))
  (bind _returnvalue_3 (- _returnvalue_2 (`self.K2_GetActorLocation`)))
  (if (<= (`KismetMathLibrary.VSize` _returnvalue_3) (`self.Range`))
    (`self.K2_SetActorLocation` (`self.Indicator`) (`KismetMathLibrary.MakeVector` (.x _returnvalue_2) (.y _returnvalue_2) 20.0) false false)
    (else
      (`self.K2_SetActorLocation` (`self.Indicator`) (`KismetMathLibrary.MakeVector` (.x (+ (* (`KismetMathLibrary.Normal` _returnvalue_3) (`self.Range`)) (`self.K2_GetActorLocation`))) (.y (+ (* (`KismetMathLibrary.Normal` _returnvalue_3) (`self.Range`)) (`self.K2_GetActorLocation`))) 20.0) false false))))

(fn `TryInteract`
  (returns (Success :type Boolean))
  (bind _job (`self.Job`))
  (bind _success (`parent.TryInteract`))
  (if _success
    (return true)
    (else
      (bind _currentjob (`self.IsWorking`))
      (if _currentjob
        (`self.InputFailed` :!label _label)
        (return false)
        (else
          (`/Engine/EditorBlueprintResources/StandardMacros.IsValid` (`self.Indicator`)
            (:`Is Valid`
              (set `self.NumFires` 0)
              (bind _returnvalue (`KismetSystemLibrary.K2_SetTimer` null "FireFireball" (`self.FireTime`) true))
              (set `self.FireTimerHandle` _returnvalue)
              (`/Game/Blueprints/Components/Job.Begin` _job)
              (`self.StartJob` _job)
              (`self.FireFireball`))
            (:`Is Not Valid`
              (goto _label))))))))

(fn `TryToStartFiring`)

(fn `UserConstructionScript`
  (`parent.UserConstructionScript`))