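; Fireball projectile that flies in an arc to a target point and deals area damage when it arrives.
; Tick advances a clamped timer, lerping from the spawn location to TargetPoint with a sine height offset scaled by RiseFactor, and faces along the movement.
; When TravelTime elapses, it spawns an impact emitter, damages overlapping Slime actors whose Health component has the matching faction, then destroys itself.
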(event `self.ReceiveBeginPlay`
  (set `self.StartingPoint` (`self.K2_GetActorLocation`)))

(event `self.ReceiveTick`
  (params (DeltaSeconds :type "Float (single-precision)"))
  (set `self.TimeTravelled` (`KismetMathLibrary.FClamp` (+ DeltaSeconds (`self.TimeTravelled`)) 0.0 (`self.TravelTime`)))
  (`self.CalculateNewLocation`)
  (if (>= (`self.TimeTravelled`) (`self.TravelTime`))
    (`self.Explode`)))

(fn `CalculateNewLocation`
  (bind _returnvalue (`KismetMathLibrary.MakeVector` (.x (`KismetMathLibrary.VLerp` (`self.StartingPoint`) (`self.TargetPoint`) (/ (`self.TimeTravelled`) (`self.TravelTime`)))) (.y (`KismetMathLibrary.VLerp` (`self.StartingPoint`) (`self.TargetPoint`) (/ (`self.TimeTravelled`) (`self.TravelTime`)))) (+ (* (`KismetMathLibrary.Sin` (* (/ (`self.TimeTravelled`) (`self.TravelTime`)) (`KismetMathLibrary.GetPI`))) (`self.RiseFactor`)) (.z (`self.TargetPoint`)) (* (- (.z (`self.StartingPoint`)) (.z (`self.TargetPoint`))) (- 1.0 (/ (`self.TimeTravelled`) (`self.TravelTime`)))))))
  (`self.K2_SetActorRotation` (`KismetMathLibrary.MakeRotFromX` (`KismetMathLibrary.Normal` (- _returnvalue (`self.K2_GetActorLocation`)))))
  (`self.K2_SetActorLocation` _returnvalue))

(fn `Explode`
  (`GameplayStatics.SpawnEmitterAtLocation` "/Game/ParticleSystems/P_ProjectileImpact.P_ProjectileImpact" (.location (`self.GetTransform`)) (.rotation (`self.GetTransform`)))
  (for _array_element (`PrimitiveComponent.GetOverlappingActors` (`self.DamageCollider`) "/Game/Blueprints/Units/Slime.Slime_C")
    (bind _returnvalue (`self.GetComponentByClass` _array_element "/Game/Blueprints/Health.Health_C"))
    (`/Engine/EditorBlueprintResources/StandardMacros.IsValid` _returnvalue
      (:`Is Valid`
        (if (`|EnumEquality` (`/Game/Blueprints/Health.Faction` _returnvalue) "NewEnumerator1")
          (`/Game/Blueprints/Health.Damage` _returnvalue (`self.Damage`))))))
  (`self.K2_DestroyActor`))

(fn `UserConstructionScript`)