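; Meteor spawner that runs recurring meteor showers while enabled, with timing and size scaled by difficulty.
; After a randomized wait, each shower spawns a random number of Meteors at staggered intervals within its box bounds.
; Each Meteor targets a random location from the first FireLocator found at BeginPlay.
; SetDifficulty derives meteor count, stagger, optional shower frequency and first-wave speed-up; CutOff is stored but unused by live logic.
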(event `self.ReceiveBeginPlay`
  (bind _outactors (`GameplayStatics.GetAllActorsOfClass` "/Game/BluePrints/Spawners/FireLocator.FireLocator_C"))
  (set `self.TargetPlane` (`|GetArrayItem` _outactors)))

(event `Enable`
  (bind _spawnspread (`self.SpawnSpread`))
  (bind _returnvalue (+ (`self.Spawn Time`) (`KismetMathLibrary.RandomFloatInRange` _spawnspread (* _spawnspread -1.0))))
  (set `self.ShowersEnabled` true)
  (`KismetSystemLibrary.Delay` (- _returnvalue (`self.beginSpeedUp`)))
  (if (`self.ShowersEnabled`) :!label _label
    (`self.Spawn Meteors`)
    (`KismetSystemLibrary.Delay` _returnvalue)
    (goto _label)))

(event `Spawn Meteors`
  (bind (_origin _boxextent) (`KismetSystemLibrary.GetComponentBounds` (`self.Box`)))
  (bind _returnvalue (`KismetMathLibrary.RandomPointInBoundingBox` _origin _boxextent))
  (set `self.Meteor Amount` (`KismetMathLibrary.RandomIntegerInRange` (`self.MeteorMin`) (`self.MeteorMax`)))
  (set `self.CurrentAmount` 0)
  (bind _returnvalue_2 (`|SpawnActorFromClass` "/Game/BluePrints/Units/Meteor.Meteor_C" (`KismetMathLibrary.MakeTransform` _returnvalue (`self.K2_GetActorRotation` self)) "Undefined" "OverrideRootScale" null null :!label _label_2))
  (`/Engine/EditorBlueprintResources/StandardMacros.IncrementInt` (`self.CurrentAmount`)
    (:`  `
      (bind _location (`/Game/BluePrints/Spawners/FireLocator.GetRandomLocation` (`self.TargetPlane`)))
      (bind _output_get (set `/Game/BluePrints/Units/Meteor.Target` _location _returnvalue_2))
      (set `/Game/BluePrints/Units/Meteor.Rotation` (`KismetMathLibrary.FindLookAtRotation` _returnvalue _output_get) _returnvalue_2)
      (if (not (>= (`self.CurrentAmount`) (`self.Meteor Amount`)))
        (`KismetSystemLibrary.Delay` (`KismetMathLibrary.RandomFloatInRange` (`self.SpawnSubMin`) (`self.SpawnSubMax`)))
        (goto _label_2)))))

(event `Disable`
  (set `self.ShowersEnabled` false))

(fn `SetCutOff`
  (params (cutOff :type "Float (double-precision)"))
  (set `self.cutOff` cutOff))

(fn `SetDifficulty`
  (params (Difficulty :type "Float (double-precision)") (AutoSetFrequency :type Boolean))
  (locals (NewLocalVar_0 :type "Float (double-precision)"))
  (bind _returnvalue (* Difficulty 0.04))
  (bind _difficulty (`local.Difficulty`))
  (bind _returnvalue_2 (- 26.0 (* (`KismetMathLibrary.FClamp` (`local.Difficulty`) 0.0 10.0) 0.3)))
  (bind _returnvalue_3 (`KismetMathLibrary.Max` (`KismetMathLibrary.FFloor` (* (- _difficulty 5.0) 1.5))))
  (`self.SetMeteorSubTime` (`KismetMathLibrary.FMax` (- 0.3 _returnvalue) 0.05) (`KismetMathLibrary.FMax` (- 0.5 _returnvalue) 0.25))
  (`self.SetMeteorAmount` (`KismetMathLibrary.Min` (+ (+ (`KismetMathLibrary.Max` (`KismetMathLibrary.FFloor` (/ (- _difficulty 2.9) 2.0))) _returnvalue_3) 2) 12) (`KismetMathLibrary.Min` (+ (+ (`KismetMathLibrary.Max` (`KismetMathLibrary.FFloor` (* _difficulty 0.61))) _returnvalue_3) 3) 14))
  (if (`local.AutoSetFrequency`)
    (`self.SetFrequency` _returnvalue_2 (/ _returnvalue_2 6.0)))
  (set `self.beginSpeedUp` (* (/ (`self.Spawn Time`) 30.0) (`KismetMathLibrary.FClamp` (`local.Difficulty`) 0.0 10.0))))

(fn `SetFrequency`
  (params (SpawnTime :type "Float (double-precision)") (SpawnSpread :type "Float (double-precision)"))
  (set `self.Spawn Time` SpawnTime)
  (set `self.SpawnSpread` SpawnSpread))

(fn `SetMeteorAmount`
  (params (Min :type Integer) (Max :type Integer))
  (set `self.MeteorMin` Min)
  (set `self.MeteorMax` Max))

(fn `SetMeteorSubTime`
  (params (Min :type "Float (double-precision)") (Max :type "Float (double-precision)"))
  (set `self.SpawnSubMin` Min)
  (set `self.SpawnSubMax` Max))

(fn `UserConstructionScript`)