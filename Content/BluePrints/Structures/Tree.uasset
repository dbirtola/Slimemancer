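; Tree structure Blueprint that topples and removes its trunk when its Health component reports a kill.
; The fall rotates TrunkRoot in a per-frame zero-delay loop until its pitch passes 40 degrees, then hands Trunk to physics.
; After a short delay, both Trunk and TrunkRoot are destroyed.
; BeginPlay also enters this fall loop, so the tree falls on spawn as well.
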(event `self.Health.OnKilled`
  ;[0 1 0.7206] Tree Cut Down
  ;[0 0.5814 1] Tree Fall
  (`SceneComponent.K2_AddLocalRotation` (`self.TrunkRoot`) (struct :`Pitch` 1.0) false false :!label _label)
  (if (<= (.pitch (`SceneComponent.RelativeRotation` (`self.TrunkRoot`))) 40.0)
    (`KismetSystemLibrary.Delay` 0.0)
    (goto _label)
    (else
      (`PrimitiveComponent.SetSimulatePhysics` (`self.Trunk`) true)
      (`KismetSystemLibrary.Delay` 2.0)
      (`ActorComponent.K2_DestroyComponent` (`self.Trunk`))
      (`ActorComponent.K2_DestroyComponent` (`self.TrunkRoot`)))))

(event `self.ReceiveBeginPlay`
  (goto _label))

(fn `UserConstructionScript`)